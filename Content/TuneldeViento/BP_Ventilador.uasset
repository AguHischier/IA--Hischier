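; Wind tunnel fan actor that pushes physics-simulating components along its up axis within a configurable box range.
; The construction script sizes and offsets the Rango box from the range variables.
; While anything overlaps it, Tick fires a grid of line traces through the volume.
; Each hit adds force at the impact point, angled between fan direction and inverted surface normal, scaled by surface alignment and falling off with distance.
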(event `self.ReceiveTick`
  (params (DeltaSeconds :type "Float (single-precision)"))
  (bind _returnvalue (`self.GetTransform`))
  (bind _returnvalue_2 (`self.GetActorUpVector`))
  (bind _distanciaentrelineas (`self.DistanciaEntreLineas`))
  (if (> (`KismetArrayLibrary.Array_Length` (`PrimitiveComponent.GetOverlappingComponents` (`self.Rango`))) 0)
    (for _index (range (+ (`KismetMathLibrary.FTrunc` (/ (`self.RangoX`) (`self.DistanciaEntreLineas`))) 1))
      (for _index_2 (range (+ (`KismetMathLibrary.FTrunc` (/ (`self.RangoY`) (`self.DistanciaEntreLineas`))) 1))
        (bind _returnvalue_3 (`KismetMathLibrary.MakeVector` (- (* _index _distanciaentrelineas) (/ (`self.RangoX`) 2.0)) (- (* _index_2 _distanciaentrelineas) (/ (`self.RangoY`) 2.0))))
        (bind (_outhit _returnvalue_4) (`KismetSystemLibrary.LineTraceSingle` (`KismetMathLibrary.TransformLocation` _returnvalue _returnvalue_3) (`KismetMathLibrary.TransformLocation` _returnvalue (+ _returnvalue_3 (`KismetMathLibrary.MakeVector` 0.0 0.0 (`self.RangoZ`)))) "TraceTypeQuery1"))
        (if _returnvalue_4
          (bind (_bblockinghit _binitialoverlap _time _distance _location _impactpoint _normal _impactnormal _physmat _hitactor _hitcomponent) (`GameplayStatics.BreakHitResult` _outhit))
          (if (`SceneComponent.IsSimulatingPhysics` _hitcomponent "None")
            (bind _returnvalue_5 (`KismetMathLibrary.NegateVector` _impactnormal))
            (`PrimitiveComponent.AddForceAtLocation` _hitcomponent (* (`KismetMathLibrary.Normal` (+ _returnvalue_2 _returnvalue_5)) (* (`KismetMathLibrary.Abs` (`KismetMathLibrary.Dot_VectorVector` _returnvalue_2 _returnvalue_5)) (* (- 1.0 _time) (`self.FuerzaMaxima`)))) _impactpoint "None")))))))

(fn `UserConstructionScript`
  (bind (_boxextent_x _boxextent_y _boxextent_z) (`KismetMathLibrary.BreakVector` (`BoxComponent.BoxExtent` (`self.Rango`))))
  (`BoxComponent.SetBoxExtent` (`self.Rango`) (`KismetMathLibrary.MakeVector` (/ (`self.RangoX`) 2.0) (/ (`self.RangoY`) 2.0) (/ (`self.RangoZ`) 2.0)) true)
  (`SceneComponent.K2_SetRelativeLocation` (`self.Rango`) (`KismetMathLibrary.MakeVector` 0.0 0.0 _boxextent_z) false false))